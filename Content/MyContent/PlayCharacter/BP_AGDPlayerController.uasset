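; Player controller that turns player input into movement, camera look, jumping and attacks for the AGD player character.
; On possess it caches the pawn as both a Character and a BP_AGDPlayerCharacter.
; Axis inputs move the pawn along its own forward and right vectors or add controller pitch and yaw.
; Jump is blocked while the character plays any montage, and primary attack is delegated to the character.
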(event EventPossess
  (params (PossessedPawn :type Pawn%20Object%20Reference))
  ;[1 1 1] on poses
  (bind _ascharacter (Utilities|Casting|CastToCharacter PossessedPawn))
  (bind _output_get (Variables|Default|SetCharacterRef _ascharacter))
  (bind _asbp_agdplayer_character (Utilities|Casting|CastToBP_AGDPlayerCharacter _output_get))
  (Variables|Default|SetPlayerRef _asbp_agdplayer_character))

(event Input|ActionEvents|InputActionJump
  (params (Key :type Key%20Structure :default "None"))
  (bind _characterref (Variables|Default|GetCharacterRef))
  ;[1 1 1] Jumping
  (:Pressed
    (bind _returnvalue (Default|IsAnyMontagePlaying (Variables|Default|GetPlayerRef)))
    (if (not _returnvalue)
      (Character|Jump _characterref)))
  (:Released
    (Character|StopJumping _characterref)))

(event Input|ActionEvents|InputActionPrimaryAttack
  (params (Key :type Key%20Structure :default "None"))
  ;[1 1 1] attack 1
  (:Pressed
    (Default|PrimaryAttack (Variables|Default|GetPlayerRef))))

(event Input|AxisEvents|InputAxisMoveForward/Backward
  (params (AxisValue :type Float%20%28single-precision%29))
  (bind _characterref (Variables|Default|GetCharacterRef))
  ;[1 1 1] Player Mov
  (Pawn|Input|AddMovementInput _characterref (Transformation|GetActorForwardVector _characterref) AxisValue false))

(event Input|AxisEvents|InputAxisMoveRight/Left
  (params (AxisValue :type Float%20%28single-precision%29))
  (bind _characterref (Variables|Default|GetCharacterRef))
  ;[1 1 1] Player Mov
  (Pawn|Input|AddMovementInput _characterref (Math|Vector|GetRightVector (Variables|/Script/Engine.Actor|GetRootComponent _characterref)) AxisValue false))

(event Input|AxisEvents|InputAxisMousePitch
  (params (AxisValue :type Float%20%28single-precision%29))
  ;[1 1 1] Player camera rotation
  (Class|PlayerController|AddPitchInput AxisValue))

(event Input|AxisEvents|InputAxisMousaeYaw
  (params (AxisValue :type Float%20%28single-precision%29))
  ;[1 1 1] Player camera rotation
  (Class|PlayerController|AddYawInput AxisValue))

(fn ConstructionScript)