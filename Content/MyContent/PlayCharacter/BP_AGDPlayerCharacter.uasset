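; Player character with melee combo attacks, a level-scaled rock-fire special ability and stat-driven levelling.
; An overlap hitbox, toggled by ActivateDamage and DeactivateDamage, applies StatsComponent base damage, while animation blueprint messages drive combo, hurt and death animations.
; Stats events spawn level-up particles, turn the character toward its attacker with a brief hurt cooldown, or reload the level on death.
; Tick gates controller-facing rotation by movement and attack state, and prints level debug text.
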(event LevelledUp(StatsComponent)
  (params (Level :type Integer) (bAreStatsInitialised :type Boolean))
  (if bAreStatsInitialised
    (Effects|SpawnEmitteratLocation "/Game/InfinityBladeEffects/Effects/FX_Ability/Heal/P_Health_Pickup_01.P_Health_Pickup_01" (Transformation|GetActorLocation))))

(event OnComponentBeginOverlap(DamageHitBox)
  (params (OverlappedComponent :type Primitive%20Component%20Object%20Reference) (OtherActor :type Actor%20Object%20Reference) (OtherComp :type Primitive%20Component%20Object%20Reference) (OtherBodyIndex :type Integer) (bFromSweep :type Boolean) (SweepResult :type Hit%20Result%20Structure%20%28by%20ref%29))
  ;[1 1 1] Apply damage to evrtng
  (Development|PrintString "damage applied")
  (if (!= OtherActor self)
    (Game|Damage|ApplyDamage OtherActor (Math|Conversions|ToFloat(Integer) (Class|AGDStatsComponent|GetBaseDamage (Variables|Default|GetStatsComponent))) 0 self "/Script/Engine.DamageType")))

(event OnHurt(StatsComponent)
  (params (IsDead :type Boolean) (Damage :type Float%20%28double-precision%29) (DamageCauser :type Actor%20Object%20Reference) (DamageType :type Damage%20Type%20Object%20Reference))
  (bind _returnvalue (Game|GetPlayerController 0))
  (if IsDead
    (Input|DisableInput _returnvalue _returnvalue)
    (Class|BIPlayerAnimations|PAnimDeath(Message) (Components|SkeletalMesh|GetAnimInstance (Variables|Character|GetMesh)))
    (Utilities|FlowControl|Delay 1.5)
    (bind _returnvalue_2 (Game|GetCurrentLevelName true))
    (Game|OpenLevel(byName) (Utilities|String|StringToName _returnvalue_2))
    (elif (not (Variables|Default|GetbRecentlyTakenDmg))
      (Variables|Default|SetbRecentlyTakenDmg true)
      (Transformation|SetActorRotation (Math|Rotator|MakeRotator 0.0 0.0 (.yaw (Math|Rotator|FindLookatRotation (Transformation|GetActorLocation) (Transformation|GetActorLocation DamageCauser)))))
      (Class|BIPlayerAnimations|PAnimTakeDamage(Message) (Components|SkeletalMesh|GetAnimInstance (Variables|Character|GetMesh)))
      (Utilities|FlowControl|Delay 0.5)
      (Variables|Default|SetbRecentlyTakenDmg false))))

(event EventTick
  (params (DeltaSeconds :type Float%20%28single-precision%29))
  (bind _statscomponent (Variables|Default|GetStatsComponent))
  (bind (_displaylevel _displayexperience) (Class|AGDStatsComponent|GetDisplayLevelInfo _statscomponent))
  (CallFunction|HandleRotation)
  (Development|PrintString (Utilities|String|ToString(Text) (Utilities|Text|FormatText "Level {level}, exp:{exp}" _displaylevel _displayexperience)) true true "(R=0.000000,G=0.660000,B=1.000000,A=1.000000)" 0.0))

(fn ConstructionScript)

(fn HandleRotation
  (Variables|/Script/Engine.CharacterMovementComponent|SetbUseControllerDesiredRotation (Variables|Character|GetCharacterMovement) (or (Math|Boolean|ANDBoolean (> (Math|Vector|VectorLength (Transformation|GetVelocity)) 0.0) (Class|AGDPlayerCharacter|GetAttackAllowed) (not (Class|AnimInstance|IsAnyMontagePlaying (Components|SkeletalMesh|GetAnimInstance (Variables|Character|GetMesh))))) (Class|AGDPlayerCharacter|GetForceRotate))))

(fn PrimaryAttack
  (Class|BIPlayerAnimations|PlayComboAttack(Message) (Components|SkeletalMesh|GetAnimInstance (Variables|Character|GetMesh)) 1.0))

(fn IsAnyMontagePlaying
  (return (Class|AnimInstance|IsAnyMontagePlaying (Components|SkeletalMesh|GetAnimInstance (Variables|Character|GetMesh)))))

(fn ActivateDamage
  (Collision|SetCollisionEnabled (Variables|Default|GetDamageHitBox) "QueryOnly"))

(fn DeactivateDamage
  (Collision|SetCollisionEnabled (Variables|Default|GetDamageHitBox) "NoCollision"))

(fn SpecialAttack
  (Game|SpawnActorfromClass "/Game/MyContent/PlayCharacter/Abilities/Ability_RockFireBurst.Ability_RockFireBurst_C" (Math|Transform|MakeTransform (Transformation|GetWorldLocation (Variables|Default|GetFeet)) "0, 0, 0" "1.000000,1.000000,1.000000") "AlwaysSpawn" "MultiplyWithRoot" self (Math|Conversions|ToFloat(Integer) (* (.DisplayLevel (Class|AGDStatsComponent|GetDisplayLevelInfo (Variables|Default|GetStatsComponent))) 11)) 0))