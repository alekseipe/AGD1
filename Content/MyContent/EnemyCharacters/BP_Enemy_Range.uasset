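; BP_Enemy_Range is an enemy character Blueprint that defines its own damage action and attack range on top of a parent class.
; When the apply-damage action event fires, it damages every GDPlayerCharacter overlapping its DamageBox, using base damage from the StatsComponent.
; Despite the Range name, the attack is an overlap check with no projectile, and the stats getter returns a short, hardcoded attack range.
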(event EventEActionApplyDamage
  (CallFunction|RangeDamage))

(fn ConstructionScript
  (|CallParentFunction))

(fn RangeDamage
  (for _array_element (Collision|GetOverlappingActors (Variables|Default|GetDamageBox) "/Script/project_1.AGDPlayerCharacter" :!class /Script/Engine.PrimitiveComponent)
    (Game|Damage|ApplyDamage _array_element (Math|Conversions|ToFloat(Integer) (Class|AGDStatsComponent|GetBaseDamage (Variables|Default|GetStatsComponent))) 0 self "/Script/Engine.DamageType")))

(fn EStatsGetAttackRange
  (return 125.0))