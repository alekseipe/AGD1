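; Enemy character that reacts to damage, dies and rewards the player with experience.
; When its StatsComponent reports a hurt, it turns to face the damage causer, is launched backward and refreshes its health bar widget.
; Animation interface messages play the hit or death reaction.
; On death it grants experience to the player's StatsComponent, waits on the death animation's returned delay, hides the bar and sets a lifespan for removal.
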(event OnHurt(StatsComponent)
  (params (IsDead :type Boolean) (Damage :type Float%20%28double-precision%29) (DamageCauser :type Actor%20Object%20Reference) (DamageType :type Damage%20Type%20Object%20Reference))
  (CallFunction|RotateandKnockBack DamageCauser)
  (CallFunction|UpdateHealthPercent)
  (if IsDead
    (CallFunction|GivePlayerExp)
    (bind _duration (Class|BIEnemyAnimations|EAnimDeath(Message) (Components|SkeletalMesh|GetAnimInstance (Variables|Character|GetMesh))))
    (Utilities|FlowControl|Delay _duration)
    (Rendering|SetVisibility (Variables|Default|GetHealthBar) false false)
    (Actor|SetLifeSpan 1e+01)
    (else
      (Class|BIEnemyAnimations|EAnimTakeDamage(Message) (Components|SkeletalMesh|GetAnimInstance (Variables|Character|GetMesh))))))

(event EventBeginPlay
  (CallFunction|UpdateHealthPercent))

(fn ConstructionScript)

(fn RotateandKnockBack
  (params (DamageCauser :type Actor%20Object%20Reference))
  (Transformation|SetActorRotation (Math|Rotator|MakeRotator 0.0 0.0 (.yaw (Math|Rotator|FindLookatRotation (Transformation|GetActorLocation) (Transformation|GetActorLocation DamageCauser)))))
  (Character|LaunchCharacter (* (Math|Vector|NegateVector (Transformation|GetActorForwardVector)) 6e+02) true false))

(fn UpdateHealthPercent
  (bind _aswui_enemy_health (Utilities|Casting|CastToWUI_EnemyHealth (UserInterface|GetWidget (Variables|Default|GetHealthBar))))
  (Default|SetHealthPercent _aswui_enemy_health (Class|AGDStatsComponent|GetHealth (Variables|Default|GetStatsComponent)) (Class|AGDStatsComponent|GetMaxHealth (Variables|Default|GetStatsComponent))))

(fn GivePlayerExp
  (bind _asbp_agdplayer_character (Utilities|Casting|CastToBP_AGDPlayerCharacter (Game|GetPlayerCharacter 0)))
  (Class|AGDStatsComponent|AddExperience (Variables|/Game/MyContent/PlayCharacter/BP_AGDPlayerCharacter.BP_AGDPlayerCharacter_C|GetStatsComponent _asbp_agdplayer_character) (Variables|Exp|GetExp)))